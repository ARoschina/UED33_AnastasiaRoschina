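; Remotely activated door, a child Blueprint whose OpenDoor event toggles it between open and closed, intended to be triggered by a button.
; After calling the parent event, it ignores requests while in motion, otherwise plays a Timeline forward or reverses it from the end.
; The Timeline scales the maximum angle to yaw DoorRotator, with a boolean choosing the swing side.
; On finish, the Timeline direction sets the open state.
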(event `self.OpenDoor`
  ;[1 1 1] Pushing the button opens the door
  (`parent.OpenDoor`)
  (if (not (`self.InProgress`))
    (if (not (`self.IsDoorOpen`))
      (bind (_direction _openprogression) (`Timeline|Timeline` :!label _label)
        (:`Update`
          (set `self.InProgress` true)
          (`SceneComponent.K2_SetRelativeRotation` (`self.DoorRotator`) (`KismetMathLibrary.MakeRotator` 0.0 0.0 (* (`self.MaxDoorOpenAngle`) _openprogression (`KismetMathLibrary.SelectFloat` -1.0 1.0 (`self.DirectionToOpenDoor`)))) false false))
        (:`Finished`
          (set `self.InProgress` false)
          (switch `ETimelineDirection` _direction
            (:`Forward`
              (set `self.IsDoorOpen` true))
            (:`Backward`
              (set `self.IsDoorOpen` false)))))
      (else
        (goto _label :!via `ReverseFromEnd`)))))

(fn `UserConstructionScript`
  (`parent.UserConstructionScript`))