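; BP_ItemBase is a base actor for interactable items that can go into a character's backpack.
; Overlapping a BP_ThirdPersonCharacter caches it, enables interaction and shows HintText, which Tick turns toward that character's FollowCamera until overlap ends.
; Interact passes the character's BP_BackpackComponent to PutIntoBackpack, an empty stub here, and returns true on every branch.
; AfterUse destroys the actor.
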(event `self.ReceiveBeginPlay`
  (`SceneComponent.SetVisibility` (`self.HintText`) false true))

(event `self.ReceiveActorBeginOverlap`
  (params (OtherActor :type "Actor Object Reference"))
  (bind _asbp_third_person_character (cast `/Game/Blueprints/Characters/BP_ThirdPersonCharacter` OtherActor))
  (set `self.CharacterInBox` _asbp_third_person_character)
  (`SceneComponent.SetVisibility` (`self.HintText`) true true)
  (set `self.Is Ready to Interact` true)
  (set `self.IsLookingAtPlayerCamera` true))

(event `self.ReceiveActorEndOverlap`
  (params (OtherActor :type "Actor Object Reference"))
  (cast `/Game/Blueprints/Characters/BP_ThirdPersonCharacter` OtherActor)
  (set `self.CharacterInBox` null)
  (`SceneComponent.SetVisibility` (`self.HintText`) false true)
  (set `self.Is Ready to Interact` false)
  (set `self.IsLookingAtPlayerCamera` false))

(event `self.ReceiveTick`
  (params (DeltaSeconds :type "Float (single-precision)"))
  (`self.LookingAtPlayerCamera`))

(fn `AfterUse`
  (`self.K2_DestroyActor`))

(fn `Interact`
  (returns (Success :type Boolean))
  (if (`self.Is Ready to Interact`)
    (bind _characterinbox (`self.CharacterInBox`)
      (:`then`
        (bind _returnvalue (`self.GetComponentByClass` _characterinbox "/Game/Blueprints/Components/BP_BackpackComponent.BP_BackpackComponent_C"))
        (`/Engine/EditorBlueprintResources/StandardMacros.IsValid` _returnvalue
          (:`Is Valid`
            (`self.PutIntoBackpack` _returnvalue)
            (return true))
          (:`Is Not Valid`
            (return true))))
      (:`else`
        (return true)))
    (else
      (return true))))

(fn `LookingAtPlayerCamera`
  (locals (L_CameraLocation :type "Vector Structure"))
  (if (`self.IsLookingAtPlayerCamera`)
    (bind _characterinbox (`self.CharacterInBox`)
      (:`then`
        (bind _asbp_third_person_character (cast `/Game/Blueprints/Characters/BP_ThirdPersonCharacter` _characterinbox))
        (set `local.L_CameraLocation` (`SceneComponent.K2_GetComponentLocation` (`/Game/Blueprints/Characters/BP_ThirdPersonCharacter.FollowCamera` _asbp_third_person_character)))
        (`SceneComponent.K2_SetWorldRotation` (`self.HintText`) (`KismetMathLibrary.FindLookAtRotation` (`SceneComponent.K2_GetComponentLocation` (`self.HintText`)) (`local.L_CameraLocation`)) false false))
      (:`else`))))

(fn `PutIntoBackpack`
  (params (InBackpack :type "/Game/Blueprints/Components/BP_BackpackComponent Object Reference")))

(fn `UserConstructionScript`)