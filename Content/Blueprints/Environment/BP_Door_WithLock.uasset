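; Lockable door child Blueprint that blocks the parent's opening while locked and shows its state with a red or green indicator light.
; Interact toggles an unlocked door open or closed.
; When locked, it unlocks without opening if the overlapped actor's BP_BackpackComponent holds every needed key name, otherwise printing "Keys needed" if a backpack exists.
; SwitchLock flips the state and refreshes the light, while Lock's logic is disconnected and never runs.
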(event `self.OpenDoor`
  (if (not (`self.IsLocked`))
    (`parent.OpenDoor`)))

(event `self.CloseDoor`
  (`parent.CloseDoor`))

(fn `DoorLightIndication`
  ;[1 1 1] Changing door light colors
  (`LightComponent.SetLightColor` (`self.LockIndicatorLight`) (`KismetMathLibrary.SelectColor` (struct :`R` 1.0 :`A` 1.0) (struct :`G` 1.0 :`B` 0.031916 :`A` 1.0) (`self.IsLocked`)) true))

(fn `Interact`
  (returns (Success :type Boolean))
  (locals (L_Backpack :type "/Game/Blueprints/Components/BP_BackpackComponent Object Reference") (L_ItemName :type Name))
  (if (`self.IsReadyToInteract`)
    (if (not (`self.IsLocked`))
      ;[1 1 1] If the door is unlocked
      (if (`self.IsDoorOpen`)
        (`self.CloseDoor`)
        (return true)
        (else
          (`self.OpenDoor`)
          (return true)))
      (else
        ;[1 1 1] If the door is locked
        (if (`KismetArrayLibrary.Array_IsValidIndex` (`self.NeededKeysName`))
          (bind _overlappedactor (`self.OverlappedActor`)
            (:`then`
              (bind _returnvalue (`self.GetComponentByClass` _overlappedactor "/Game/Blueprints/Components/BP_BackpackComponent.BP_BackpackComponent_C"))
              (`/Engine/EditorBlueprintResources/StandardMacros.IsValid` _returnvalue
                (:`Is Valid`
                  (set `local.L_Backpack` _returnvalue)
                  (for _array_element (`self.NeededKeysName`)
                    (bind _output_get (set `local.L_ItemName` _array_element))
                    (if (`BlueprintSetLibrary.Set_Contains` (`/Game/Blueprints/Components/BP_BackpackComponent.Items` (`local.L_Backpack`)) _output_get)
                      (`/Engine/EditorBlueprintResources/StandardMacros.IncrementInt` (`self.UsedItemIncrement`))))
                  (if (== (`self.UsedItemIncrement`) (`KismetArrayLibrary.Array_Length` (`self.NeededKeysName`)))
                    (`self.Unlock`)
                    (set `self.UsedItemIncrement` 0)
                    (else
                      (`KismetSystemLibrary.PrintString` "Keys needed" true false (struct :`R` 0.541667 :`B` 0.030692 :`A` 1.0))
                      (return true))))
                (:`Is Not Valid`
                  (return true))))
            (:`else`
              (return true)))
          (else
            (return true)))))
    (else
      (return false))))

(fn `Lock`)

(fn `SwitchLock`
  (set `self.IsLocked` (not (`self.IsLocked`)))
  (`self.DoorLightIndication`))

(fn `Unlock`
  (set `self.IsLocked` false)
  (`self.DoorLightIndication`))

(fn `UserConstructionScript`
  (`parent.UserConstructionScript`)
  (`self.DoorLightIndication`))