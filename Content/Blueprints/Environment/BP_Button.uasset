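; Interactable push button that opens a list of linked doors in the environment.
; Actor overlap toggles a hint text, and Interact calls Push, which ignores repeat presses while the animation runs.
; A timeline slides the button body along Z, then calls OpenDoor on each entry in DoorsToOpen when it finishes.
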(event `self.ReceiveBeginPlay`
  ;[1 1 1] Show hint text when player is near
  (`SceneComponent.SetVisibility` (`self.HintText`) false true))

(event `self.ReceiveActorBeginOverlap`
  (params (OtherActor :type "Actor Object Reference"))
  ;[1 1 1] Show hint text when player is near
  (`SceneComponent.SetVisibility` (`self.HintText`) true true)
  (set `self.Is Ready to Interact` (`self.Is Ready To Interact`)))

(event `self.ReceiveActorEndOverlap`
  (params (OtherActor :type "Actor Object Reference"))
  ;[1 1 1] Show hint text when player is near
  (`SceneComponent.SetVisibility` (`self.HintText`) false true)
  (set `self.Is Ready to Interact` false))

(event `Push`
  (if (not (`self.InProgress`))
    (bind (_direction _move) (`Timeline|Timeline_0` :!via `PlayFromStart`)
      (:`Update`
        (set `self.InProgress` true)
        (`SceneComponent.K2_SetRelativeLocation` (`self.ButtonBodyMesh`) (`KismetMathLibrary.MakeVector` 0.0 0.0 (* (`self.MaxButtonOffset`) _move)) false false))
      (:`Finished`
        (set `self.InProgress` false)
        (`self.DoorsOpenMechanism`)))))

(fn `DoorsOpenMechanism`
  (if (`KismetArrayLibrary.Array_IsValidIndex` (`self.DoorsToOpen`))
    (for _array_element (`self.DoorsToOpen`)
      (if true
        (`/Game/Blueprints/Environment/BP_DoorBase.OpenDoor` _array_element)))))

(fn `Interact`
  (returns (Success :type Boolean))
  (`self.Push`)
  (return true))

(fn `UserConstructionScript`)